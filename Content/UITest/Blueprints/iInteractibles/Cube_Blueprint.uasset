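; An interactable physics cube that the player can pick up and drop, with a description pop-up widget.
; Interact attaches it to the hand's CubeHolder socket with physics off and the widget visible, or detaches it, restoring physics and hiding the widget.
; Player overlap with the trigger box calls the widget's show and hide pop-up functions.
; While visible, the widget turns on yaw only to face the camera each tick.
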(event `self.ReceiveTick`
  (params (DeltaSeconds :type "Float (single-precision)"))
  ;[1 1 1] UI Rotator Blueprint
  (if (`SceneComponent.bVisible` (`self.ShowDesUI`))
    (`self.UpdatePopUpFacing`)))

(event `self.TriggerBox.OnComponentBeginOverlap`
  (params (OverlappedComponent :type "PrimitiveComponent Object Reference") (OtherActor :type "Actor Object Reference") (OtherComp :type "PrimitiveComponent Object Reference") (OtherBodyIndex :type Integer) (bFromSweep :type Boolean) (SweepResult :type "HitResult Structure (by ref)"))
  ;[1 1 1] PopUp UI
  (if (== OtherActor (`GameplayStatics.GetPlayerPawn` 0))
    (bind _aswm_show_des_ui (cast `/Game/UITest/UI/WM_ShowDesUI` (`WidgetComponent.GetUserWidgetObject` (`self.ShowDesUI`))))
    (`/Game/UITest/UI/WM_ShowDesUI.ShowPopUp` _aswm_show_des_ui)))

(event `self.TriggerBox.OnComponentEndOverlap`
  (params (OverlappedComponent :type "PrimitiveComponent Object Reference") (OtherActor :type "Actor Object Reference") (OtherComp :type "PrimitiveComponent Object Reference") (OtherBodyIndex :type Integer))
  ;[1 1 1] PopUp UI
  (if (== OtherActor (`GameplayStatics.GetPlayerPawn` 0))
    (bind _aswm_show_des_ui (cast `/Game/UITest/UI/WM_ShowDesUI` (`WidgetComponent.GetUserWidgetObject` (`self.ShowDesUI`))))
    (`/Game/UITest/UI/WM_ShowDesUI.HidePopUp` _aswm_show_des_ui)))

(event `/Game/UITest/Blueprints/iInteractible.Interact`
  (params (Hand :type "SceneComponent Object Reference") (bHolding :type Boolean))
  ;[1 1 1] PickUp & Drop Objects
  (if bHolding
    (`PrimitiveComponent.SetSimulatePhysics` (`self.StaticMeshComponent`) false)
    (`self.K2_AttachToComponent` Hand "CubeHolder" "KeepWorld" "KeepWorld" "KeepWorld")
    (`SceneComponent.SetVisibility` (`self.ShowDesUI`) true false)
    (else
      (`self.K2_DetachFromActor` "KeepWorld" "KeepWorld" "KeepWorld")
      (`PrimitiveComponent.SetSimulatePhysics` (`self.StaticMeshComponent`) true)
      (`SceneComponent.SetVisibility` (`self.ShowDesUI`) false false))))

(fn `UpdatePopUpFacing`
  (bind (_returnvalue_roll _returnvalue_pitch _returnvalue_yaw) (`KismetMathLibrary.BreakRotator` (`KismetMathLibrary.FindLookAtRotation` (`SceneComponent.K2_GetComponentLocation` (`self.ShowDesUI`)) (`PlayerCameraManager.GetCameraLocation` (`GameplayStatics.GetPlayerCameraManager` 0)))))
  (`SceneComponent.K2_SetWorldRotation` (`self.ShowDesUI`) (`KismetMathLibrary.MakeRotator` 0.0 0.0 _returnvalue_yaw) false false))

(fn `UserConstructionScript`)